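; C4 explosive actor that shows a blast as an expanding sphere and knocks physics objects away.
; Explode swaps the model to a translucent sphere, scales it up over a timeline, and destroys the actor after a half-second delay started from the timeline update.
; Any physics-simulating component overlapping the model receives a radial velocity impulse from its location, with no check for whether Explode has run.
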(event `self.ReceiveBeginPlay`)

(event `Explode`
  (bind _model (`self.Model`))
  (`StaticMeshComponent.SetStaticMesh` _model "/Engine/EngineMeshes/Sphere.Sphere")
  (`PrimitiveComponent.SetMaterial` _model 0 "/Engine/EngineDebugMaterials/M_SimpleTranslucent.M_SimpleTranslucent")
  (bind (_direction _newtrack_0) (`Timeline|Timeline` :!via `PlayFromStart`)
    (:`Update`
      (`SceneComponent.SetWorldScale3D` (`self.Model`) (`KismetMathLibrary.Conv_DoubleToVector` _newtrack_0))
      (`KismetSystemLibrary.Delay` 0.5)
      (`self.K2_DestroyActor`))))

(event `self.Model.OnComponentBeginOverlap`
  (params (OverlappedComponent :type "PrimitiveComponent Object Reference") (OtherActor :type "Actor Object Reference") (OtherComp :type "PrimitiveComponent Object Reference") (OtherBodyIndex :type Integer) (bFromSweep :type Boolean) (SweepResult :type "HitResult Structure (by ref)"))
  (if (`SceneComponent.IsSimulatingPhysics` OtherComp "None")
    (`PrimitiveComponent.AddRadialImpulse` OtherComp (`SceneComponent.K2_GetComponentLocation` (`self.Model`)) 20000.0 500.0 "RIF_Constant" true)))

(fn `UserConstructionScript`)