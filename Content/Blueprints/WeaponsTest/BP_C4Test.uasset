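; BP_C4Test is a test C4 explosive actor that is pushed forward when spawned and can be detonated.
; On BeginPlay it applies a small impulse to its static mesh along the mesh's forward vector.
; Its Boom function activates and fires a RadialForce impulse, spawns BP_Explosion at the mesh transform and destroys the actor.
; Nothing in this Blueprint calls Boom, so detonation relies on an external trigger.
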(event `self.ReceiveBeginPlay`
  (bind _staticmesh (`self.StaticMesh`))
  (`PrimitiveComponent.AddImpulse` _staticmesh (* (`SceneComponent.GetForwardVector` _staticmesh) 20.0) "None" false))

(event `self.ReceiveTick`
  (params (DeltaSeconds :type "Float (single-precision)")))

(fn `Boom`
  (bind _radialforce (`self.RadialForce`))
  (`ActorComponent.Activate` _radialforce true)
  (`|SpawnActorFromClass` "/Game/Blueprints/WeaponsTest/BP_Explosion.BP_Explosion_C" (`SceneComponent.K2_GetComponentToWorld` (`self.StaticMesh`)) "Undefined" "MultiplyWithRoot" null null)
  (`RadialForceComponent.FireImpulse` _radialforce)
  (`self.K2_DestroyActor`))

(fn `UserConstructionScript`)