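; Test grenade actor that launches itself on spawn and explodes after a short fuse.
; BeginPlay applies a forward impulse to the static mesh, then waits a fixed delay before calling Boom.
; Boom activates the RadialForce component, fires its impulse to push nearby physics objects, and destroys the actor.
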(event `self.ReceiveBeginPlay`
  (bind _staticmesh (`self.StaticMesh`))
  (`PrimitiveComponent.AddImpulse` _staticmesh (* (`SceneComponent.GetForwardVector` _staticmesh) 2500.0) "None" false)
  (`KismetSystemLibrary.Delay` 5.0)
  (`self.Boom`))

(event `self.ReceiveTick`
  (params (DeltaSeconds :type "Float (single-precision)")))

(fn `Boom`
  (bind _radialforce (`self.RadialForce`))
  (`ActorComponent.Activate` _radialforce false)
  (`RadialForceComponent.FireImpulse` _radialforce)
  (`self.K2_DestroyActor`))

(fn `UserConstructionScript`)