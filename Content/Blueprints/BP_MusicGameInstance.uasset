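; BP_MusicGameInstance, named as a game instance, plays background music that persists across level transitions.
; PlayGameMusic spawns the given 2D sound on its first call and stores the audio component in Music.
; Later calls with a valid Sound go through ForIsValid, which spawns only if Music is not playing.
; An invalid Sound loops back to the first-call spawn path, replacing the Music reference without a playback check.
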(event `ForIsValid`
  (params (Sound :type "SoundBase Object Reference"))
  (if (not (`AudioComponent.IsPlaying` (`self.Music`)))
    (bind _returnvalue (`GameplayStatics.SpawnSound2D` Sound 1.0 1.0 0.0 null true))
    (set `self.Music` _returnvalue)))

(event `PlayGameMusic`
  (params (Sound :type "SoundBase Object Reference"))
  (if (`self.IsFirstTime`)
    (bind _returnvalue (`GameplayStatics.SpawnSound2D` Sound 1.0 1.0 0.0 null true :!label _label))
    (set `self.Music` _returnvalue)
    (set `self.IsFirstTime` false)
    (else
      (`/Engine/EditorBlueprintResources/StandardMacros.IsValid` Sound
        (:`Is Valid`
          (`self.ForIsValid` Sound))
        (:`Is Not Valid`
          (goto _label))))))